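; BP_JLE_RuntimeLoader is an actor that replaces level spawn markers with real actors when play begins.
; On BeginPlay it gathers every BP_JLE_SpawnMarker and looks up each marker's AssetId in its AssetIds array.
; The matching index picks a class from the parallel SpawnClasses array, which spawns at the marker's transform before the marker is destroyed.
; Unknown IDs only print a message, alongside debug prints of each ID and index.
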(event `self.ReceiveBeginPlay`
  (bind _outactors (`GameplayStatics.GetAllActorsOfClass` "/Game/JLE/BP_JLE_SpawnMarker.BP_JLE_SpawnMarker_C"))
  (for _array_element _outactors
    (bind _asbp_jle_spawn_marker (cast `/Game/JLE/BP_JLE_SpawnMarker` _array_element))
    (bind _assetid (`/Game/JLE/BP_JLE_SpawnMarker.AssetId` _asbp_jle_spawn_marker))
    (`KismetSystemLibrary.PrintString` _assetid)
    (bind _returnvalue (`KismetArrayLibrary.Array_Find` (`self.AssetIds`) _assetid))
    (`KismetSystemLibrary.PrintString` (`KismetStringLibrary.Conv_IntToString` _returnvalue))
    (if (>= _returnvalue 0)
      (`|SpawnActorFromClass` (`|GetArrayItem` (`self.SpawnClasses`) _returnvalue) (`self.GetTransform` _asbp_jle_spawn_marker) "Undefined" "MultiplyWithRoot" null null)
      (`self.K2_DestroyActor` _asbp_jle_spawn_marker)
      (else
        (`KismetSystemLibrary.PrintString` "Unknown AssetId")))))

(fn `UserConstructionScript`)