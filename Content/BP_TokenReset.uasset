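; BP_TokenReset restores arcade tokens in the level to a visible state with collision enabled.
; ResetArcadeTokens finds every actor of TokenActorClass, unhides it and re-enables its collision, printing an error if the class is unset.
; It also makes each primitive component and its children visible and sets the component's collision to query-only.
; Nothing in this Blueprint calls the reset; BeginPlay only clears PlayerActor.
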(event `self.ReceiveBeginPlay`
  (set `self.PlayerActor` null))

(fn `ResetArcadeTokens`
  (if (`KismetSystemLibrary.IsValidClass` (`self.TokenActorClass`))
    (bind _outactors (`GameplayStatics.GetAllActorsOfClass` (`self.TokenActorClass`)))
    (for _array_element _outactors
      (`self.SetActorHiddenInGame` _array_element false)
      (`self.SetActorEnableCollision` _array_element true)
      (for _array_element_2 (`self.K2_GetComponentsByClass` _array_element "/Script/Engine.PrimitiveComponent")
        (`SceneComponent.SetVisibility` _array_element_2 true true)
        (`SceneComponent.SetHiddenInGame` _array_element_2 false true)
        (`PrimitiveComponent.SetCollisionEnabled` _array_element_2 "QueryOnly")))
    (else
      (`KismetSystemLibrary.PrintString` "BP_TokenReset: TokenActorClass is not set"))))

(fn `UserConstructionScript`)